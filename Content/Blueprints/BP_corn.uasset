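; BP_corn is an AI pawn that wanders randomly and moves toward the player once its PawnSensing component sees a pawn.
; Any sighting latches IsSeeingPlayer on and starts an AI move toward player 0.
; Tick issues moves to random reachable points after short random delays, pausing only while IsSeeingPlayer and Moving are both true.
; Either move clears Moving when it ends, but only wandering sets it.
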(event `self.PawnSensing.OnSeePawn`
  (params (Pawn :type "Pawn Object Reference"))
  (set `self.isSeeingPlayer` true)
  (`self.FollowPlayer`))

(event `FollowPlayer`
  (if (`self.isSeeingPlayer`)
    (`|AIMoveTo` self (0.0 0.0 0.0) (`GameplayStatics.GetPlayerCharacter` 0) 100.0
      (:`OnSuccess`
        _)
      (:`OnFail`
        _))
    (set `self.Moving` false)
    (else
      (set `self.isSeeingPlayer` false))))

(event `self.ReceiveTick`
  (params (DeltaSeconds :type "Float (single-precision)"))
  ;[1 1 1] AI Random Movement
  (if (not (and (`self.isSeeingPlayer`) (`self.Moving`)))
    (`KismetSystemLibrary.Delay` (`KismetMathLibrary.RandomFloatInRange` 1.0 3.0))
    (set `self.Moving` true)
    (`|AIMoveTo` self (`NavigationSystemV1.K2_GetRandomReachablePointInRadius` (`self.K2_GetActorLocation`) 10000.0 null null) null 100.0
      (:`OnSuccess`
        _)
      (:`OnFail`
        _))
    (set `self.Moving` false)))

(fn `UserConstructionScript`)