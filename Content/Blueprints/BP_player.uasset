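; BP_player is the player pawn, providing first-person-style movement, mouse look and a toggleable flashlight.
; Mouse axes feed controller yaw and inverted pitch, while move axes add input along the capsule's forward and right vectors.
; The F key drives a FlipFlop that shows and hides the SpotLight component.
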(event `InputAxisKey|MouseX`
  (params (AxisValue :type "Float (single-precision)"))
  (`self.AddControllerYawInput` AxisValue))

(event `InputAxisKey|MouseY`
  (params (AxisValue :type "Float (single-precision)"))
  (`self.AddControllerPitchInput` (* AxisValue -1.0)))

(event `InputAxis|Move Forward / Backward`
  (params (AxisValue :type "Float (single-precision)"))
  (`self.AddMovementInput` (`SceneComponent.GetForwardVector` (`self.CapsuleComponent`)) AxisValue))

(event `InputAxis|Move Right / Left`
  (params (AxisValue :type "Float (single-precision)"))
  (`self.AddMovementInput` (`SceneComponent.GetRightVector` (`self.CapsuleComponent`)) AxisValue))

(event `Key|F`
  (params (Key :type "Key Structure"))
  (:`Pressed`
    (`/Engine/EditorBlueprintResources/StandardMacros.FlipFlop`
      (:`A`
        (`SceneComponent.SetVisibility` (`self.SpotLight`) true true))
      (:`B`
        (`SceneComponent.SetVisibility` (`self.SpotLight`) false true)))))

(fn `UserConstructionScript`)